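; Scene actor that becomes the player's view, showcases configurable "yellow object" meshes, and starts a Movie Render Queue job for MainSequence on BeginPlay.
; Camera activation applies the clip path, background, lights, white-material fallback, visible object and transform.
; Tick optionally rotates EmptyObject and lerps object positions.
; Pixel Streaming JSON input, keyed by Category and Item, swaps meshes and level-sequence clips or remaps values into rotation, scale and position.
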(event OnComponentActivated(Camera)
  (params (Component :type Actor%20Component%20Object%20Reference) (bReset :type Boolean))
  (Utilities|FlowControl|Sequence
    (:then_0
      (bind _output_get (Variables|Default|SetImageMediaFileRef "/Game/YellowObjects/VideoSource_Request/MS_Clip1.MS_Clip1"))
      (Class|ImgMediaSource|SetSequencePath _output_get (Variables|Default|GetClipPath))
      (Rendering|SetVisibility (Variables|Default|GetPlane) (Variables|Default|GetbBackground) false)
      (Rendering|SetVisibility (Variables|Default|GetPointLight) (Variables|Default|GetbLight1) false)
      (Rendering|SetVisibility (Variables|Default|GetPointLight1) false (Variables|Default|GetbLight2)))
    (:then_1
      (if (not (Variables|Default|GetbMask))
        (Utilities|MaterialWhite)))
    (:then_2
      (switch int (Variables|Default|GetYellowObjectNum)
        (:Default
          (CallFunction|Switch2 :!label _label))
        (:0
          (CallFunction|Switch1 :!label _label_2))
        (:1
          (goto _label_2))
        (:2
          (goto _label))
        (:3
          (CallFunction|Switch3))
        (:4
          (CallFunction|Switch4))))
    (:then_3
      (if (Variables|Default|GetbCustomPosition)
        (Transformation|SetRelativeLocation (Variables|Default|GetYellowObject) (Math|Vector|MakeVector (Variables|Default|GetPosition_X) (Variables|Default|GetPosition_Y) (Variables|Default|GetPosition_Z)) false false)))
    (:then_4
      (if true
        (Transformation|SetRelativeScale3D (Variables|Default|GetYellowObject) (Math|Vector|MakeVector (Variables|Default|GetScale_X) (Variables|Default|GetScale_Y) (Variables|Default|GetScale_Z)))))))

(event Custom|Switch1
  (Rendering|SetVisibility (Variables|Default|GetYellowObject1) true true)
  (Rendering|SetVisibility (Variables|Default|GetYellowObject) false true))

(event Custom|Switch2
  (Rendering|SetVisibility (Variables|Default|GetYellowObject) true true)
  (Rendering|SetVisibility (Variables|Default|GetYellowObject1) false true))

(event Custom|OnRenderingFinished
  (params (PipelineExecutor :type Movie%20Pipeline%20Executor%20Base%20Object%20Reference) (bSuccess :type Boolean))
  (EventDispatchers|UnbindEventfromOnExecutorFinishedDelegate PipelineExecutor (delegate Custom|OnRenderingFinished))
  (Development|PrintString "Yes, MoviePipeline, Finished!"))

(event Custom|Switch3
  (Rendering|SetVisibility (Variables|Default|GetYellowObject2) true true)
  (Rendering|SetVisibility (Variables|Default|GetYellowObject1) false true))

(event Custom|Switch4
  (Rendering|SetVisibility (Variables|Default|GetYellowObject3) true true)
  (Rendering|SetVisibility (Variables|Default|GetYellowObject1) false true))

(event Custom|OnJSONEvent
  (params (Descriptor :type String))
  (Variables|Default|SetDescriptor Descriptor)
  (Utilities|PixelStreamingUpdate))

(event EventBeginPlay
  (Utilities|FlowControl|Sequence
    (:then_0
      (Game|Player|SetViewTargetwithBlend (Game|GetPlayerController 0) self 0.0 "VTBlend_Linear" 0.0 false)
      (Rendering|SetActorHiddenInGame (Game|Player|GetPlayerPawn 0) true)
      (Utilities|FlowControl|Sequence
        (:then_0
          (bind _returnvalue (Game|ConstructObjectfromClass "/Script/MovieRenderPipelineCore.MoviePipelineQueue" self))
          (bind _output_get (Variables|Default|SetActiveQueue _returnvalue))
          (bind _returnvalue_2 (Class|MoviePipelineQueue|AllocateNewJob _output_get "/Script/MovieRenderPipelineCore.MoviePipelineExecutorJob"))
          (Variables|/Script/MovieRenderPipelineCore.MoviePipelineExecutorJob|SetSequence _returnvalue_2 (Utilities|MakeSoftObjectPath "/Game/YellowObjects/SequenceSetup/MainSequence.MainSequence"))
          (Variables|/Script/MovieRenderPipelineCore.MoviePipelineExecutorJob|SetMap _returnvalue_2 (Utilities|MakeSoftObjectPath "/Game/Main.Main"))
          (Class|MoviePipelineExecutorJob|SetConfiguration _returnvalue_2 "/Game/Cinematics/MoviePipeline/Presets/MoviePipelineMasterConfig.MoviePipelineMasterConfig"))
        (:then_1
          (bind _returnvalue_3 (Game|ConstructObjectfromClass "/Script/MovieRenderPipelineCore.MoviePipelineInProcessExecutor" (|MoviePipelineQueueEngineSubsystem)))
          (Variables|/Script/MovieRenderPipelineCore.MoviePipelineInProcessExecutor|SetbUseCurrentLevel _returnvalue_3 true)
          (EventDispatchers|AssignOnExecutorFinishedDelegate _returnvalue_3 (delegate Custom|OnRenderingFinished))
          (Class|MoviePipelineExecutorBase|Execute _returnvalue_3 (Variables|Default|GetActiveQueue))
          (Class|MoviePipelineQueueEngineSubsystem|RenderQueuewithExecutor (|MoviePipelineQueueEngineSubsystem) "/Script/MovieRenderPipelineEditor.MoviePipelinePIEExecutor"))))
    (:then_1
      (EventDispatchers|AssignOnInputEvent (Variables|Default|GetPixelStreamerInput) (delegate Custom|OnJSONEvent)))))

(event EventTick
  (params (DeltaSeconds :type Float%20%28single-precision%29))
  (Utilities|FlowControl|Sequence
    (:then_1
      (if (Variables|Default|GetbRotate)
        _))
    (:then_2
      (if (Variables|Default|GetbLightsRotation)
        (Transformation|AddLocalRotation (Variables|Default|GetEmptyObject) (Math|Rotator|MakeRotator (Variables|Default|GetLightRotation_X) (Variables|Default|GetLightRotation_Y) (Variables|Default|GetLightRotation_Z)) false false)))
    (:then_3
      (if (Variables|Default|GetbAnimateObject)
        (Variables|Default|SetAnimLerp (+ (Variables|Default|GetAnimLerp) (Variables|Default|GetAnimIncrease)))
        (Transformation|SetRelativeLocation (Variables|Default|GetYellowObject) (Math|Vector|Lerp(Vector) (Math|Vector|MakeVector (Variables|Default|GetAnimStartPosition_X) (Variables|Default|GetAnimStartPosition_Y) (Variables|Default|GetAnimStartPosition_Z)) (Math|Vector|MakeVector (Variables|Default|GetAnimEndPosition_X) (Variables|Default|GetAnimEndPosition_Y) (Variables|Default|GetAnimEndPosition_Z)) (Variables|Default|GetAnimLerp)) false false)))))

(event EventEndPlay
  (params (EndPlayReason :type EEndPlayReason%20Enum :default "Destroyed"))
  (switch Utilities|FlowControl|Switch|SwitchonEEndPlayReason EndPlayReason
    (:Destroyed
      _)
    (:LevelTransition
      _)
    (:EndPlayInEditor
      _)
    (:RemovedFromWorld
      _)
    (:Quit
      _))
  (Development|PrintString "Quitting Editor from Python"))

(fn ConstructionScript)